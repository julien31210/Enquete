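; Locked door that opens when its OpenDoor event finds at least one key on the player character.
; Opening uses up a key, destroys the held item, swings the door mesh on a timeline with sound and gamepad rumble, then removes the Box component.
; Without a key, a still-closed door plays a positional locked sound and briefly shows a UIText warning, guarded by a flag against stacking.
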(event Custom|OpenDoor
  (bind _asmain_player_character_bp (Utilities|Casting|CastToMainPlayerCharacter_BP (Game|GetPlayerCharacter 0)))
  (if (>= (Variables|/Game/01_BLUEPRINT/MainPlayerCharacter_BP.MainPlayerCharacter_BP_C|GetnbrCle _asmain_player_character_bp) 1)
    (bind _result (Math|Integer|DecrementInt (Variables|/Game/01_BLUEPRINT/MainPlayerCharacter_BP.MainPlayerCharacter_BP_C|GetnbrCle _asmain_player_character_bp))
      (:%20%20
        (Variables|/Game/01_BLUEPRINT/MainPlayerCharacter_BP.MainPlayerCharacter_BP_C|SetnbrCle _asmain_player_character_bp _result)
        (bind _asmain_player_character_bp_2 (Utilities|Casting|CastToMainPlayerCharacter_BP (Game|GetPlayerCharacter 0)))
        (Actor|DestroyActor (Variables|/Game/01_BLUEPRINT/MainPlayerCharacter_BP.MainPlayerCharacter_BP_C|GetCurrentHeldItem _asmain_player_character_bp_2))
        (Development|PrintString "Ouverture de la porte")
        (Utilities|FlowControl|Sequence
          (:then_0
            (Audio|PlaySound2D "/Game/04_SOUND_DESIGN/Ouverture_Porte.Ouverture_Porte" 1.0 1.0 0.0 0 0))
          (:then_1
            (bind _newtrack_0 (Timeline|OpeningDoor Play)
              (:Update
                (Transformation|SetRelativeRotation (Variables|Default|GetP_Porte_Low) (Math|Rotator|MakeRotator 0.0 0.0 (* _newtrack_0 -9e+01)) false false))))
          (:then_2
            (Game|Feedback|PlayDynamicForceFeedback (Game|GetPlayerController 0) 0.5 1.0 true true true true))
          (:then_3
            (Components|DestroyComponent (Variables|Default|GetBox))
            (Variables|Default|SetalrdOpen true)))))
    (elif (not (Variables|Default|GetalrdOpen))
      (Development|PrintString "Vous avez besoin d'une clé")
      (Audio|PlaySoundatLocation "/Game/04_SOUND_DESIGN/Locked_Door.Locked_Door" (Transformation|GetWorldLocation (Variables|Default|GetP_Porte_Low)) "0, 0, 0" 1.0 1.0 0.0 "/Game/04_SOUND_DESIGN/NewSoundAttenuation.NewSoundAttenuation" 0 0)
      (if (not (Variables|Default|GettextAlrdy))
        (Variables|Default|SettextAlrdy true)
        (Utilities|Casting|CastToMainPlayerCharacter_BP (Game|GetPlayerCharacter 0))
        (bind _returnvalue (UserInterface|CreateWidget "/Game/09_UI/UIText.UIText_C"))
        (UserInterface|Viewport|AddtoViewport _returnvalue 0)
        (Variables|/Game/09_UI/UIText.UIText_C|SetlockedDoor _returnvalue true)
        (Utilities|FlowControl|Delay 3.0)
        (Widget|RemovefromParent _returnvalue)
        (Variables|Default|SettextAlrdy false)
        (Variables|/Game/09_UI/UIText.UIText_C|SetlockedDoor _returnvalue false)))))

(fn ConstructionScript)
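; SteamDoor_BP is a door that swings open when its IfIsRepaired event fires.
; The 90degresDoor flag selects one of two timelines, Timeline_0 when true or OponningDoorSteam otherwise.
; The chosen timeline's track, scaled by RotationAngle, drives the relative yaw of the PPorteLow component on each update.
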(event Custom|IfIsRepaired
  (if (Variables|Default|Get90degresDoor)
    (bind _newtrack_0 (Timeline|Timeline_0 Play)
      (:Update
        (Transformation|SetRelativeRotation (Variables|Default|GetP_Porte_Low) (Math|Rotator|MakeRotator 0.0 0.0 (* _newtrack_0 (Variables|Default|GetRotationAngle))) false false)))
    (else
      (bind _newtrack_0_2 (Timeline|OponningDoorSteam Play)
        (:Update
          (Transformation|SetRelativeRotation (Variables|Default|GetP_Porte_Low) (Math|Rotator|MakeRotator 0.0 0.0 (* _newtrack_0_2 (Variables|Default|GetRotationAngle))) false false))))))

(fn ConstructionScript)
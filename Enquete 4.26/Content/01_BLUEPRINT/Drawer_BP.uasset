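; Drawer actor that slides drawer meshes open or shut and lets the player pick up a note to read.
; Its OppenDrawer event line-traces from the player camera to find the hit static mesh component.
; An object-name match on ItemNote shows a reading widget; otherwise the mesh's relative Y selects opening or closing.
; Timelines lerp the mesh along Y with matching sounds, while CanOpen blocks retriggering during the slide.
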(event Custom|OppenDrawer
  (bind _returnvalue (Transformation|GetActorLocation))
  (if (Variables|Default|GetCanOpen)
    (Variables|Default|SetCanOpen false)
    (bind _asmain_player_character_bp (Utilities|Casting|CastToMainPlayerCharacter_BP (Game|GetPlayerCharacter 0)))
    (bind (_outhit _returnvalue_2) (Collision|LineTraceForObjects (Transformation|GetWorldLocation (Variables|/Game/01_BLUEPRINT/MainPlayerCharacter_BP.MainPlayerCharacter_BP_C|GetCamera _asmain_player_character_bp)) (+ (Transformation|GetWorldLocation (Variables|/Game/01_BLUEPRINT/MainPlayerCharacter_BP.MainPlayerCharacter_BP_C|GetCamera _asmain_player_character_bp)) (* (Math|Vector|GetForwardVector (Variables|/Game/01_BLUEPRINT/MainPlayerCharacter_BP.MainPlayerCharacter_BP_C|GetCamera _asmain_player_character_bp)) 5e+02)) (Utilities|Array|MakeArray "ObjectTypeQuery2") false 0 "None" false))
    (if _returnvalue_2
      (bind _asstatic_mesh_component (Utilities|Casting|CastToStaticMeshComponent (.HitComponent (Collision|BreakHitResult _outhit))))
      (bind _output_get (Variables|Default|SetStaticMeshRef _asstatic_mesh_component))
      ;[1 1 1] Pick a note
      (if (Utilities|Enum|Equal(Enum) (Utilities|GetObjectName 0) "ItemNote")
        (Variables|Default|SetHoldingNote? true)
        (bind _returnvalue_3 (UserInterface|CreateWidget "/Game/09_UI/ReadingNote.ReadingNote_C"))
        (bind _output_get_2 (Variables|Default|SetNoteRef _returnvalue_3))
        (UserInterface|Viewport|AddtoViewport _output_get_2 0)
        (elif (not (>= (.y (Variables|/Script/Engine.SceneComponent|GetRelativeLocation _asstatic_mesh_component)) 45.0))
          (Audio|PlaySoundatLocation "/Game/04_SOUND_DESIGN/Tiroir_en_bois_ouverture.Tiroir_en_bois_ouverture" _returnvalue "0, 0, 0" 1.0 1.0 0.0 0 0 0)
          (Variables|Default|SetStartLoc (Math|Vector|MakeVector (.x (Variables|/Script/Engine.SceneComponent|GetRelativeLocation (Variables|Default|GetStaticMeshRef))) (.y (Variables|/Script/Engine.SceneComponent|GetRelativeLocation (Variables|Default|GetStaticMeshRef))) (.z (Variables|/Script/Engine.SceneComponent|GetRelativeLocation (Variables|Default|GetStaticMeshRef)))))
          (Variables|Default|SetEndLoc (Math|Vector|MakeVector (.x (Variables|/Script/Engine.SceneComponent|GetRelativeLocation (Variables|Default|GetStaticMeshRef))) (+ (.y (Variables|/Script/Engine.SceneComponent|GetRelativeLocation (Variables|Default|GetStaticMeshRef))) 45.0) (.z (Variables|/Script/Engine.SceneComponent|GetRelativeLocation (Variables|Default|GetStaticMeshRef)))))
          (bind _opendrwer (Timeline|OpenDrawer PlayFromStart)
            (:Update
              (Transformation|SetRelativeLocation (Variables|Default|GetStaticMeshRef) (Math|Vector|Lerp(Vector) (Variables|Default|GetStartLoc) (Variables|Default|GetEndLoc) _opendrwer) false false))
            (:Finished
              (Variables|Default|SetCanOpen true)))
          (else
            (Audio|PlaySoundatLocation "/Game/04_SOUND_DESIGN/Tiroir_en_bois_fermeture.Tiroir_en_bois_fermeture" _returnvalue "0, 0, 0" 1.0 1.0 0.0 0 0 0)
            (Variables|Default|SetStartLoc (Math|Vector|MakeVector (.x (Variables|/Script/Engine.SceneComponent|GetRelativeLocation (Variables|Default|GetStaticMeshRef))) (.y (Variables|/Script/Engine.SceneComponent|GetRelativeLocation (Variables|Default|GetStaticMeshRef))) (.z (Variables|/Script/Engine.SceneComponent|GetRelativeLocation (Variables|Default|GetStaticMeshRef)))))
            (Variables|Default|SetEndLoc (Math|Vector|MakeVector (.x (Variables|/Script/Engine.SceneComponent|GetRelativeLocation (Variables|Default|GetStaticMeshRef))) (- (.y (Variables|/Script/Engine.SceneComponent|GetRelativeLocation (Variables|Default|GetStaticMeshRef))) 45.0) (.z (Variables|/Script/Engine.SceneComponent|GetRelativeLocation (Variables|Default|GetStaticMeshRef)))))
            (bind _opendrwer_2 (Timeline|Timeline_0 PlayFromStart)
              (:Update
                (Transformation|SetRelativeLocation (Variables|Default|GetStaticMeshRef) (Math|Vector|Lerp(Vector) (Variables|Default|GetStartLoc) (Variables|Default|GetEndLoc) _opendrwer_2) false false))
              (:Finished
                (Variables|Default|SetCanOpen true))))))
      (else
        (Variables|Default|SetCanOpen true)))))

(event EventBeginPlay
  (Input|EnableInput (Game|GetPlayerController 0)))

(fn ConstructionScript)
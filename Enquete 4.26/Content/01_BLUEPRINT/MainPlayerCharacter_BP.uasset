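; Touch-controlled first-person player character that creates the HUD, looks around by finger drag and walks to a double-tapped point on the NavMesh.
; Each tick, camera traces highlight note items, and CheckLookAt tracks the nearby BP_Interface actor under the view, sending it a look-at message.
; The Loot action messages that actor and also runs separate long-range traces with casts to loot notes, fuel generators with fuzes, repair pipes and open doors.
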(event EventTick
  (params (DeltaSeconds :type Float%20%28single-precision%29))
  (bind _returnvalue (Game|GetPlayerController 0))
  (bind _finderindex (Variables|Default|GetFinderIndex))
  (bind _camera (Variables|Default|GetCamera))
  (bind (_locationx _locationy _biscurrentlypressed) (Class|PlayerController|GetInputTouchState _returnvalue _finderindex))
  (bind _returnvalue_2 (Transformation|GetWorldLocation _camera))
  (Utilities|FlowControl|Sequence
    (:then_0
      ;[1 1 1] HighLight Item
      (bind (_outhit _returnvalue_3) (Collision|LineTraceByChannel _returnvalue_2 (+ _returnvalue_2 (* (Math|Vector|GetForwardVector _camera) 5e+03)) "TraceTypeQuery1" false 0 "ForOneFrame"))
      (if _returnvalue_3
        (bind _asitem_notes (Utilities|Casting|CastToItemNotes (.HitActor (Collision|BreakHitResult _outhit))))
        (Default|HighLight _asitem_notes)))
    (:then_1
      ;[1 1 1] Rotation Camera
      (if _biscurrentlypressed
        (if (Variables|Default|GetisTouching)
          (Pawn|Input|AddControllerYawInput (/ (- _locationx (Variables|Default|GetX)) 1e+01))
          (Pawn|Input|AddControllerPitchInput (/ (- _locationy (Variables|Default|GetY)) 1e+01))
          (Variables|Default|SetX _locationx)
          (Variables|Default|SetY _locationy)
          (else
            (Variables|Default|SetisTouching true)
            (Variables|Default|SetX _locationx)
            (Variables|Default|SetY _locationy)))
        (else
          (Variables|Default|SetisTouching false))))
    (:then_2
      (CallFunction|CheckLookat))))

(event EventBeginPlay
  (bind _returnvalue (UserInterface|CreateWidget "/Game/09_UI/HUD.HUD_C" (Game|GetPlayerController 0)))
  (UserInterface|Viewport|AddtoViewport _returnvalue 0))

(event Input|ActionEvents|InputActionLoot
  (params (Key :type Key%20Structure :default "None"))
  (:Pressed
    (bind _lookatactor (Variables|Default|GetLookAtActor)
      (:then
        (Class|BPInterface|Interactwith(Message) _lookatactor self))
      (:else))))

(event Input|ActionEvents|InputActionLoot
  (params (Key :type Key%20Structure :default "None"))
  (bind _camera (Variables|Default|GetCamera))
  (bind _returnvalue (Transformation|GetWorldLocation _camera))
  ;[1 1 1] Open Door
  (:Pressed
    (bind (_outhit _returnvalue_2) (Collision|LineTraceByChannel _returnvalue (+ _returnvalue (* (Math|Vector|GetForwardVector _camera) 5e+03)) "TraceTypeQuery1" false 0 "None"))
    (if _returnvalue_2
      (bind _askey_door_bp (Utilities|Casting|CastToKeyDoor_BP (.HitActor (Collision|BreakHitResult _outhit))))
      (Default|OpenDoor _askey_door_bp))))

(event Input|ActionEvents|InputActionLoot
  (params (Key :type Key%20Structure :default "None"))
  (bind _camera (Variables|Default|GetCamera))
  (bind _returnvalue (Transformation|GetWorldLocation _camera))
  ;[1 1 1] Looting Notes
  (:Pressed
    (bind (_outhit _returnvalue_2) (Collision|LineTraceByChannel _returnvalue (+ _returnvalue (* (Math|Vector|GetForwardVector _camera) 5e+03)) "TraceTypeQuery1" false 0 "None"))
    (if _returnvalue_2
      (bind _asitem_notes (Utilities|Casting|CastToItemNotes (.HitActor (Collision|BreakHitResult _outhit))))
      (Default|LootItem _asitem_notes)
      (Audio|PlaySound2D "/Game/04_SOUND_DESIGN/Take_a_note.Take_a_note" 1.0 1.0 0.0 0 0))))

(event Input|ActionEvents|InputActionLoot
  (params (Key :type Key%20Structure :default "None"))
  (bind _camera (Variables|Default|GetCamera))
  (bind _returnvalue (Transformation|GetWorldLocation _camera))
  ;[1 1 1] Interact With Generator
  (:Pressed
    (bind (_outhit _returnvalue_2) (Collision|LineTraceByChannel _returnvalue (+ _returnvalue (* (Math|Vector|GetForwardVector _camera) 5e+03)) "TraceTypeQuery1" false 0 "None"))
    (if _returnvalue_2
      (bind _asgenerator_bp (Utilities|Casting|CastToGenerator_BP (.HitActor (Collision|BreakHitResult _outhit))))
      (Default|AddFuzetoGen _asgenerator_bp))))

(event Input|ActionEvents|InputActionLoot
  (params (Key :type Key%20Structure :default "None"))
  (bind _camera (Variables|Default|GetCamera))
  (bind _returnvalue (Transformation|GetWorldLocation _camera))
  ;[1 1 1] Reparing Cable
  (:Pressed
    (bind (_outhit _returnvalue_2) (Collision|LineTraceByChannel _returnvalue (+ _returnvalue (* (Math|Vector|GetForwardVector _camera) 5e+03)) "TraceTypeQuery1" false 0 "None"))
    (if _returnvalue_2
      (bind _asbroken_pipe_bp (Utilities|Casting|CastToBrokenPipe_BP (.HitActor (Collision|BreakHitResult _outhit))))
      (Default|RepairPipe _asbroken_pipe_bp))))

(event Input|TouchEvents|InputTouch
  (params (Location :type Vector) (FingerIndex :type ETouchIndex%20Enum))
  ;[1 1 1] Rotation Camera
  (:Moved
    (Variables|Default|SetFinderIndex FingerIndex)))

(event Input|TouchEvents|InputTouch
  (params (Location :type Vector) (FingerIndex :type ETouchIndex%20Enum))
  (bind _returnvalue (Game|GetPlayerController 0))
  ;[1 1 1] Double Tap
  (:Pressed
    (bind _output_get (Variables|Default|SetTap (+ (Variables|Default|GetTap) 1)))
    (if (>= _output_get 2)
      ;[1 1 1] Move To NavMesh
      (AI|Navigation|SimpleMovetoLocation _returnvalue (.Location (Collision|BreakHitResult (.HitResult (Class|PlayerController|GetHitResultUnderFingerbyChannel _returnvalue "Touch1" "TraceTypeQuery1" true)))))
      (Audio|PlaySound2D "/Game/04_SOUND_DESIGN/Marche_-_Beton.Marche_-_Beton" 1.0 1.0 0.0 0 0)))
  (:Released
    (Utilities|FlowControl|Delay 0.25)
    (Variables|Default|SetTap 0)))

(fn ConstructionScript)

(fn CheckLookat
  (bind _camera (Variables|Default|GetCamera))
  (bind _returnvalue (Transformation|GetWorldLocation _camera))
  (bind _outhit (Collision|LineTraceByChannel _returnvalue (+ (* (Math|Vector|GetForwardVector (Transformation|GetWorldRotation _camera)) 2.5e+02) _returnvalue) "TraceTypeQuery1" false 0 "ForOneFrame"))
  (if (Utilities|DoesObjectImplementInterface (.hitactor _outhit) "/Game/01_BLUEPRINT/BP_Interface.BP_Interface_C")
    (if (not (== (.hitactor _outhit) (Variables|Default|GetLookAtActor)))
      (bind _output_get (Variables|Default|SetLookAtActor (.hitactor _outhit)))
      (Class|BPInterface|Lookat(Message) _output_get self)
      (Utilities|FlowControl|Sequence
        (:then_0
          (return (Variables|Default|GetLookAtActor)))
        (:then_1
          (Variables|Default|SetactualyHolding true)
          (return (Variables|Default|GetLookAtActor)))))
    (else
      (bind _output_get_2 (Variables|Default|SetLookAtActor 0))
      (return _output_get_2))))
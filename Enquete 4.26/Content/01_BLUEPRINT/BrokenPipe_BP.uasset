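; BrokenPipe_BP is a broken pipe that the player repairs with a roll of tape (scotch).
; RepairPipe checks the player character's NbrScotch count, printing a message when it is empty.
; On success it decrements the count, shows the Cylinder1 mesh hidden at BeginPlay, and destroys the player's held item.
; It then calls IfIsRepaired on a Target reference and hides the steam effect.
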(event Custom|RepairPipe
  (bind _asmain_player_character_bp (Utilities|Casting|CastToMainPlayerCharacter_BP (Game|GetPlayerCharacter 0)))
  (if (>= (Variables|/Game/01_BLUEPRINT/MainPlayerCharacter_BP.MainPlayerCharacter_BP_C|GetnbrScotch _asmain_player_character_bp) 1)
    (bind _output_get (Variables|/Game/01_BLUEPRINT/MainPlayerCharacter_BP.MainPlayerCharacter_BP_C|SetnbrScotch _asmain_player_character_bp (Variables|/Game/01_BLUEPRINT/MainPlayerCharacter_BP.MainPlayerCharacter_BP_C|GetnbrScotch _asmain_player_character_bp)))
    (Math|Integer|DecrementInt _output_get
      (:%20%20
        (Rendering|SetVisibility (Variables|Default|GetCylinder1) true false)
        (bind _asmain_player_character_bp_2 (Utilities|Casting|CastToMainPlayerCharacter_BP (Game|GetPlayerCharacter 0)))
        (Actor|DestroyActor (Variables|/Game/01_BLUEPRINT/MainPlayerCharacter_BP.MainPlayerCharacter_BP_C|GetCurrentHeldItem _asmain_player_character_bp_2))
        (Default|IfIsRepaired (Variables|Default|GetTarget))
        (Rendering|SetVisibility (Variables|Default|GetSteam_FX) false false)))
    (else
      (Development|PrintString "Pas de scotch"))))

(event EventBeginPlay
  (Rendering|SetVisibility (Variables|Default|GetCylinder1) false false))

(fn ConstructionScript)
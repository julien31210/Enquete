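; Generator actor that the player powers by inserting two fuses, starting its steam effect.
; AddFuzeToGen reveals one hidden fuse mesh per call, spending the player's fuse count through UseFuze, which destroys the held item when none remain.
; The second fuse shows steam, triggers force feedback, and optionally notifies a steam door target or powers a broken pipe, starting its steam and engine sound.
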(event Custom|AddFuzeToGen
  (bind _brokenpipe (Variables|Default|GetBrokenPipe))
  (if (Variables|Default|GetoneIsOn)
    (if (not (Variables|Default|GettwoIsOn))
      (bind _asmain_player_character_bp (Utilities|Casting|CastToMainPlayerCharacter_BP (Game|GetPlayerCharacter 0)))
      (if (>= (Variables|/Game/01_BLUEPRINT/MainPlayerCharacter_BP.MainPlayerCharacter_BP_C|GetnbrFuze _asmain_player_character_bp) 1)
        (Rendering|SetVisibility (Variables|Default|GetFuze3) true false)
        (Rendering|SetVisibility (Variables|Default|GetSteam_FX) true false)
        (CallFunction|UseFuze)
        (Variables|Default|SettwoIsOn true)
        (Game|Feedback|PlayDynamicForceFeedback (Game|GetPlayerController 0) 1.0 1.0 true true true true)
        (Utilities|FlowControl|Sequence
          (:then_0
            (if (Variables|Default|GetisSteamDoor%20?)
              (Default|IfIsRepaired (Variables|Default|GetTarget))))
          (:then_1
            (if (Variables|Default|GetneedToRepairePipe?)
              (Variables|/Game/01_BLUEPRINT/BrokenPipe_BP.BrokenPipe_BP_C|SetisPowered? _brokenpipe true)
              (Default|StartSteam _brokenpipe)
              (Audio|PlaySoundatLocation "/Game/04_SOUND_DESIGN/Steam_Engine.Steam_Engine" (Transformation|GetWorldLocation (Variables|Default|GetP_Generateur)) "0, 0, 0" 1.0 1.0 0.0 "/Game/04_SOUND_DESIGN/NewSoundAttenuation.NewSoundAttenuation" 0 0))))))
    (else
      (bind _asmain_player_character_bp_2 (Utilities|Casting|CastToMainPlayerCharacter_BP (Game|GetPlayerCharacter 0)))
      (if (>= (Variables|/Game/01_BLUEPRINT/MainPlayerCharacter_BP.MainPlayerCharacter_BP_C|GetnbrFuze _asmain_player_character_bp_2) 1)
        (Rendering|SetVisibility (Variables|Default|GetFuze2) true false)
        (CallFunction|UseFuze)
        (Variables|Default|SetoneIsOn true)))))

(event Custom|UseFuze
  (bind _asmain_player_character_bp (Utilities|Casting|CastToMainPlayerCharacter_BP (Game|GetPlayerCharacter 0)))
  (if (> (Variables|/Game/01_BLUEPRINT/MainPlayerCharacter_BP.MainPlayerCharacter_BP_C|GetnbrFuze _asmain_player_character_bp) 0)
    (Math|Integer|DecrementInt (Variables|/Game/01_BLUEPRINT/MainPlayerCharacter_BP.MainPlayerCharacter_BP_C|GetnbrFuze _asmain_player_character_bp)
      (:%20%20
        (if (<= (Variables|/Game/01_BLUEPRINT/MainPlayerCharacter_BP.MainPlayerCharacter_BP_C|GetnbrFuze _asmain_player_character_bp) 0)
          (bind _asmain_player_character_bp_2 (Utilities|Casting|CastToMainPlayerCharacter_BP (Game|GetPlayerCharacter 0)))
          (Actor|DestroyActor (Variables|/Game/01_BLUEPRINT/MainPlayerCharacter_BP.MainPlayerCharacter_BP_C|GetCurrentHeldItem _asmain_player_character_bp_2))
          (Game|Feedback|PlayDynamicForceFeedback (Game|GetPlayerController 0) 0.5 0.1 true true true true)
          (Audio|PlaySound2D "/Game/04_SOUND_DESIGN/Placer_Fusible.Placer_Fusible" 1.0 1.0 0.0 0 0))))))

(event Custom|DeletUsedItem
  (bind _asmain_player_character_bp (Utilities|Casting|CastToMainPlayerCharacter_BP (Game|GetPlayerCharacter 0)))
  (Actor|DestroyActor (Variables|/Game/01_BLUEPRINT/MainPlayerCharacter_BP.MainPlayerCharacter_BP_C|GetCurrentHeldItem _asmain_player_character_bp)))

(event EventBeginPlay
  (Rendering|SetVisibility (Variables|Default|GetFuze2) false false)
  (Rendering|SetVisibility (Variables|Default|GetSteam_FX) false false))

(fn ConstructionScript)